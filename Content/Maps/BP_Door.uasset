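; A double door actor that swings open after about five seconds of accumulated interaction, tracked as a percentage.
; While its widget exists, Tick turns it toward the player camera and advances DoorPercent through a Gate toggled by GateOpen and GateClose.
; At full progress, a DoOnce calls AnimateDoor and destroys the widget.
; AnimateDoor uses a timeline to rotate both leaves in opposite directions, or reverses it if DoorClosed is false.
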(event Custom|AnimateDoor
  ;[1 1 1] 애니매이션
  (if (Variables|Default|GetDoorClosed)
    (bind _door_open (Timeline|Door%20Rotation PlayFromStart)
      (:Update
        (Transformation|SetRelativeLocationAndRotation (Variables|Default|GetDoorL) "-80.000000, 0, 0" (Math|Rotator|MakeRotator 0.0 0.0 _door_open) false false)
        (Transformation|SetRelativeLocationAndRotation (Variables|Default|GetDoorR) "80.000000, 0, 0" (* (Math|Rotator|MakeRotator 0.0 0.0 _door_open) -1.0) false false)))
    (else
      (Timeline|Door%20Rotation Reverse))))

(event Custom|GateClose
  ;[1 1 1] 상호작용
  (Utilities|FlowControl|Gate true) ; enters at Close
)

(event Custom|FacePercent
  (bind _returnvalue (Game|GetPlayerCameraManager 0))
  (bind _returnvalue_2 (Camera|GetCameraRotation _returnvalue))
  (Transformation|SetWorldRotation (Variables|Default|GetWidget) (Math|Rotator|MakeRotator (+ (.roll _returnvalue_2) 1.8e+02) (+ (.pitch _returnvalue_2) 1.8e+02) (.yaw _returnvalue_2)) false false))

(event Custom|Set%20Percent
  ;[1 1 1] 퍼센트
  (bind _output_get (Variables|Default|SetDoorPercent (+ (/ (Utilities|Time|GetWorldDeltaSeconds) 5.0) (Variables|Default|GetDoorPercent))))
  (if (>= _output_get 1.0)
    (Utilities|FlowControl|DoOnce false
      (:Completed
        (CallFunction|AnimateDoor)
        (Components|DestroyComponent (Variables|Default|GetWidget))))))

(event Custom|GateOpen
  ;[1 1 1] 상호작용
  (Utilities|FlowControl|Gate true) ; enters at Open
)

(event EventTick
  (params (DeltaSeconds :type Float%20%28single-precision%29))
  ;[1 1 1] 상호작용
  (Utilities|IsValid (Variables|Default|GetWidget)
    (:Is%20Valid
      (CallFunction|FacePercent)
      (Utilities|FlowControl|Gate true
        (:Exit
          (CallFunction|SetPercent))))))

(fn ConstructionScript)