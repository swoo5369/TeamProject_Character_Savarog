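; BP_Skill3 is a self-timed effect actor for Sevarog's third skill, made of a decal and a particle system.
; On BeginPlay, a custom event waits briefly, then a timeline curve scales the decal relative to its DecalScale.
; A few seconds later, a second timeline scales the particle system from an enlarged base size.
; The actor destroys itself after a final delay, with no damage or collision logic in its graphs.
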(event Custom|DecalScaleUp
  (Utilities|FlowControl|Delay 1.0)
  (bind _새_트랙_0 (Timeline|타임라인_0 PlayFromStart)
    (:Update
      (Transformation|SetWorldScale3D (Variables|Default|GetDecal) (* (Variables|Default|GetDecalScale) _새_트랙_0)))))

(event Custom|ScaleParticle
  (bind _새_트랙_0 (Timeline|타임라인_1 PlayFromStart)
    (:Update
      (Transformation|SetWorldScale3D (Variables|Default|GetParticleSystem) (* "5.000000,5.000000,5.000000" _새_트랙_0)))))

(event EventBeginPlay
  (CallFunction|DecalScaleUp)
  (Utilities|FlowControl|Delay 3.0)
  (CallFunction|ScaleParticle)
  (Utilities|FlowControl|Delay 3.5)
  (Actor|DestroyActor))

(fn ConstructionScript)