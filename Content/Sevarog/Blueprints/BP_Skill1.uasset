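; BP_Skill1 is Sevarog's targeted area-damage skill actor, with a decal and an overlap sphere.
; It follows the cursor's ground position at a fixed height until Attack input locks the location and requests the cast through a server call.
; The cast plays the player's skill motion, spawns a particle actor, removes the decal, then briefly enables sphere overlaps to damage Monster-tagged actors before destroying itself.
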(event OnComponentBeginOverlap(Sphere)
  (params (OverlappedComponent :type Primitive%20Component%20Object%20Reference) (OtherActor :type Actor%20Object%20Reference) (OtherComp :type Primitive%20Component%20Object%20Reference) (OtherBodyIndex :type Integer) (bFromSweep :type Boolean) (SweepResult :type Hit%20Result%20Structure%20%28by%20ref%29))
  (if (Actor|ActorHasTag OtherActor "Monster")
    (Game|Damage|ApplyDamage OtherActor (Variables|Default|GetSkill%20Damage) 0 0)))

(event Custom|UseSkill
  (Utilities|FlowControl|Sequence
    (:then_0
      (Default|Skill1Motion (.AsBP%20Player%20Savarog (Utilities|Casting|CastToBP_Player_Savarog (Game|GetPlayerCharacter 0)))))
    (:then_1
      (Utilities|FlowControl|Delay 0.3)
      (Game|SpawnActorfromClass "/Game/Sevarog/Blueprints/BP_Skill1_Particle.BP_Skill1_Particle_C" (Math|Transform|MakeTransform (Variables|Default|GetSkillLocation) "0, 0, 0" "1,1,1") "AlwaysSpawn" self 0)
      (Components|DestroyComponent (Variables|Default|GetDecal))
      (Utilities|FlowControl|Delay 0.5)
      (Variables|/Script/Engine.PrimitiveComponent|SetbGenerateOverlapEvents (Variables|Default|GetSphere) true)
      (Utilities|FlowControl|Delay 0.1)
      (Actor|DestroyActor))))

(event Custom|Skill_Server
  (CallFunction|UseSkill))

(event EventBeginPlay
  (Variables|/Script/Engine.PrimitiveComponent|SetbGenerateOverlapEvents (Variables|Default|GetSphere) false))

(event EventTick
  (params (DeltaSeconds :type Float%20%28single-precision%29))
  (Utilities|FlowControl|Gate false
    (:Exit
      (CallFunction|FollowMouse))))

(event Input|AxisEvents|InputAxisAttack
  (params (AxisValue :type Float%20%28single-precision%29))
  (if (> AxisValue 0.0)
    (Utilities|FlowControl|DoOnce false
      (:Completed
        (Variables|Default|SetSkillLocation (Transformation|GetActorLocation))
        (Utilities|FlowControl|Sequence
          (:then_0
            (Utilities|FlowControl|Gate false) ; enters at Close
          )
          (:then_1
            (CallFunction|SkillServer)))))))

(fn ConstructionScript)

(fn FollowMouse
  (bind _returnvalue (Game|GetPlayerController 0))
  (bind _hitresult (Game|Player|GetHitResultUnderCursorbyChannel _returnvalue "TraceTypeQuery1" true))
  (bind _location (Collision|BreakHitResult _hitresult))
  (Transformation|SetActorLocation (Math|Vector|MakeVector (.x _location) (.y _location) 2e+01) false false))